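; SimpleSky_BP drives a day/night cycle by rotating a referenced Sun actor over a configurable day length in minutes.
; BeginPlay converts that length into seconds per game hour.
; Each Tick advances an unwrapped Hour counter, maps it to a sun pitch with a 90-degree offset, then has the SkySphere update its sun direction to match.
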(event EventBeginPlay
  (bind _output_get (Variables|Default|SetOneDay (* (Variables|Default|GetDayLengthInMinutes) 6e+01)))
  (Variables|Default|SetOneHour (/ _output_get 24.0)))

(event Collision|EventActorBeginOverlap
  (params (OtherActor :type Actor%20Object%20Reference)))

(event EventTick
  (params (DeltaSeconds :type Float%20%28single-precision%29))
  (bind _output_get (Variables|Default|SetHour (+ (Variables|Default|GetHour) (/ DeltaSeconds (Variables|Default|GetOneHour)))))
  (bind _output_get_2 (Variables|Default|SetSunAngle (+ (* (/ _output_get 6.0) 9e+01) 9e+01)))
  (Transformation|SetActorRotation (Variables|Default|GetSun) (Math|Rotator|MakeRotator 0.0 _output_get_2 0.0))
  (Default|UpdateSunDirection (Variables|Default|GetSkySphere)))

(fn ConstructionScript)